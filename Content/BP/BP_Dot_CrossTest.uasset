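; Test actor that visualizes dot and cross product math between three spheres.
; On BeginPlay, the Dot timeline moves Sphere2 along X each update.
; The normalized Sphere1-to-Sphere2 and Sphere1-to-Sphere3 directions feed a dot product, shown on TextRender as cosine and arccosine in degrees and radians.
; A debug line trace runs from Sphere1 to the unnormalized cross product, used directly as a world position.
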(event `self.ReceiveBeginPlay`
  (bind _returnvalue (`SceneComponent.K2_GetComponentLocation` (`self.Sphere1`)))
  (bind _returnvalue_2 (`KismetMathLibrary.Dot_VectorVector` (`KismetMathLibrary.Normal` (- (`SceneComponent.K2_GetComponentLocation` (`self.Sphere2`)) (`SceneComponent.K2_GetComponentLocation` (`self.Sphere1`)))) (`KismetMathLibrary.Normal` (- (`SceneComponent.K2_GetComponentLocation` (`self.Sphere3`)) (`SceneComponent.K2_GetComponentLocation` (`self.Sphere1`))))))
  (bind (_direction _newtrack_0) (`Timeline|Dot` :!via `PlayFromStart`)
    (:`Update`
      (`SceneComponent.K2_AddWorldOffset` (`self.Sphere2`) (* (`KismetMathLibrary.MakeVector` (.x _newtrack_0) (.y _newtrack_0) (.z _newtrack_0)) (-3.0 0.0 0.0)) false false)
      (`TextRenderComponent.K2_SetText` (`self.TextRender`) (`KismetTextLibrary.Conv_StringToText` (`KismetStringLibrary.Concat_StrStr` "ACOSd:" (`KismetStringLibrary.Conv_DoubleToString` (`KismetMathLibrary.DegAcos` _returnvalue_2)) " ACOS:" (`KismetStringLibrary.Conv_DoubleToString` (`KismetMathLibrary.Acos` _returnvalue_2)) " COS:" (`KismetStringLibrary.Conv_DoubleToString` _returnvalue_2))))
      ;[1 1 1] 叉积
      (`KismetSystemLibrary.LineTraceSingle` :`Start` _returnvalue :`End` (`KismetMathLibrary.Cross_VectorVector` (- (`SceneComponent.K2_GetComponentLocation` (`self.Sphere2`)) _returnvalue) (- (`SceneComponent.K2_GetComponentLocation` (`self.Sphere3`)) (`SceneComponent.K2_GetComponentLocation` (`self.Sphere1`)))) :`TraceChannel` "TraceTypeQuery1" :`DrawDebugType` "ForDuration" :`DrawTime` 0.0))))

(fn `UserConstructionScript`)
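; BP_ADAS is a Blueprint that applies an ADAS road line test material to two static mesh components.
; On BeginPlay it creates one dynamic material instance, stores it as MADAS and assigns it to both meshes.
; Tick and the construction script do nothing, as their sine-driven "c3" parameter animation and duplicate material setup are disconnected.
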(event `self.ReceiveBeginPlay`
  (bind _returnvalue (`PrimitiveComponent.CreateDynamicMaterialInstance` (`self.StaticMesh1`) 0 "/Game/Developers/ADS/ADAS/Material/M_ADASRoadLine_Test_Inst.M_ADASRoadLine_Test_Inst" "None"))
  (bind _output_get (set `self.M_ADAS` _returnvalue))
  (`PrimitiveComponent.SetMaterial` (`self.StaticMesh1`) 0 _output_get)
  (`PrimitiveComponent.SetMaterial` (`self.StaticMesh`) 0 _output_get))

(event `self.ReceiveTick`
  (params (DeltaSeconds :type "Float (single-precision)")))

(fn `UserConstructionScript`)
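; BP_Collision is a trigger actor that shows a WBP_ShowRT widget while the third-person character is inside its Box.
; On begin overlap it casts the other actor to BP_ThirdPersonCharacter, then creates the widget for player 0, adds it to the viewport and stores it in ShowRTUI.
; On end overlap by that character it removes the stored widget and clears the reference; other actors entering only print a cast-failure message.
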(event `self.Box.OnComponentBeginOverlap`
  (params (OverlappedComponent :type "PrimitiveComponent Object Reference") (OtherActor :type "Actor Object Reference") (OtherComp :type "PrimitiveComponent Object Reference") (OtherBodyIndex :type Integer) (bFromSweep :type Boolean) (SweepResult :type "HitResult Structure (by ref)"))
  (cast `/Game/ThirdPerson/Blueprints/BP_ThirdPersonCharacter` OtherActor
    (:`then`
      (bind _returnvalue (`|CreateWidget` "/Game/UI/WBP_ShowRT.WBP_ShowRT_C" (`GameplayStatics.GetPlayerController` 0)))
      (`UserWidget.AddToViewport` _returnvalue 0)
      (set `self.ShowRT_UI` _returnvalue))
    (:`CastFailed`
      (`KismetSystemLibrary.PrintString` "Cast Faild"))))

(event `self.Box.OnComponentEndOverlap`
  (params (OverlappedComponent :type "PrimitiveComponent Object Reference") (OtherActor :type "Actor Object Reference") (OtherComp :type "PrimitiveComponent Object Reference") (OtherBodyIndex :type Integer))
  (cast `/Game/ThirdPerson/Blueprints/BP_ThirdPersonCharacter` OtherActor)
  (`Widget.RemoveFromParent` (`self.ShowRT_UI`))
  (set `self.ShowRT_UI` null))

(fn `UserConstructionScript`)
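; BP_BrushSnow is a brush that stamps its world position into the interactive snow canvases as it moves.
; On BeginPlay it caches the level's BP_Canvas and BP_FluidCanvas actors.
; Each Tick it traces a short distance down from a Z-offset point on the Visibility channel.
; On a hit it adds a brush to BP_Canvas with the hit distance as height, plus a fixed-size, zero-height brush to the fluid canvas.
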(event `self.ReceiveBeginPlay`
  (bind _returnvalue (`GameplayStatics.GetActorOfClass` "/Game/Material/RenderTarget/InteractSnow/BP_Canvas.BP_Canvas_C"))
  (set `self.Brush` _returnvalue)
  (bind _returnvalue_2 (`GameplayStatics.GetActorOfClass` "/Game/Material/Fluid/BP_FluidCanvas.BP_FluidCanvas_C"))
  (set `self.FluidBrush` _returnvalue_2))

(event `self.ReceiveTick`
  (params (DeltaSeconds :type "Float (single-precision)"))
  (bind (_x _y _z) (`KismetMathLibrary.BreakVector3f` (`self.K2_GetComponentLocation` self)))
  (bind _returnvalue (`KismetMathLibrary.MakeVector` _x _y (+ _z (`self.Center_Z_OffSet`))))
  (bind (_x_2 _y_2 _z_2) (`KismetMathLibrary.BreakVector3f` _returnvalue))
  (bind (_outhit _returnvalue_2) (`KismetSystemLibrary.LineTraceSingle` _returnvalue (`KismetMathLibrary.MakeVector` _x_2 _y_2 (- _z_2 30.0)) "TraceTypeQuery1"))
  (if _returnvalue_2
    (`/Game/Material/RenderTarget/InteractSnow/BP_Canvas.AddBrush` (`self.Brush`) (make `/Game/Material/RenderTarget/InteractSnow/S_BrushInfo` _returnvalue (`self.Brush Info Size`) (`.Distance` (`GameplayStatics.BreakHitResult` _outhit))))
    (`/Game/Material/Fluid/BP_FluidCanvas.AddBrush` (`self.FluidBrush`) (make `/Game/Material/RenderTarget/InteractSnow/S_BrushInfo` _returnvalue (5.0 5.0)))))
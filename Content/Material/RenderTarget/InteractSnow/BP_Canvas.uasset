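; Snow canvas actor that keeps a player-centered render target of deformations for interactive snow, publishing its position and size through MPC_Snow.
; Each tick it copies RT_Snow to RT_SnowSave, redraws it through an offset material to compensate for player movement, then stamps queued brushes with height-driven material.
; M_Accumulation is then drawn into RT_SnowSave.
; The second target avoids sampling while drawing; post-physics ticking lets brushes register first.
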(event `self.ReceiveBeginPlay`
  (`KismetRenderingLibrary.ClearRenderTarget2D` "/Game/Material/RenderTarget/InteractSnow/RT_Snow.RT_Snow")
  (`KismetRenderingLibrary.ClearRenderTarget2D` "/Game/Material/RenderTarget/InteractSnow/RT_SnowSave.RT_SnowSave")
  (bind _returnvalue (`KismetMaterialLibrary.CreateDynamicMaterialInstance` "/Game/Material/RenderTarget/InteractSnow/M_OffSet.M_OffSet"))
  (set `self.OffSetSnow` _returnvalue)
  (bind _returnvalue_2 (`KismetMaterialLibrary.CreateDynamicMaterialInstance` "/Game/Material/RenderTarget/InteractSnow/M_DrawMaterial.M_DrawMaterial"))
  (set `self.DrawSnowMaterial` _returnvalue_2))

(event `self.ReceiveActorBeginOverlap`
  (params (OtherActor :type "Actor Object Reference")))

(event `self.ReceiveTick`
  (params (DeltaSeconds :type "Float (single-precision)"))
  (bind _snowheight (`self.SnowHeight`))
  (bind _drawsnowmaterial (`self.DrawSnowMaterial`))
  (bind (_returnvalue_x _returnvalue_y) (`KismetMathLibrary.BreakVector2D` (/ (- (`self.Position`) (`self.LastPosition`)) (`self.CanvasSize`))))
  ;[1 1 1] class default中tick group设置为物理之后，以确保在添加笔刷之后再进行绘制
  ;[1 1 1] 更新位置，是绘制效果以角色为中心
  (`self.UpdatePosition` (`KismetMathLibrary.Conv_VectorToVector2D` (`self.K2_GetActorLocation` (`GameplayStatics.GetPlayerPawn` 0))))
  ;[1 1 1] RT无法在绘制的同时采样，所以用另一张RT暂存当前帧的RT，再绘制到当前帧RT上，以保存之前绘制内容
  (`self.CopySnowRT`)
  (`KismetRenderingLibrary.ClearRenderTarget2D` "/Game/Material/RenderTarget/InteractSnow/RT_Snow.RT_Snow")
  (`MaterialInstanceDynamic.SetVectorParameterValue` (`self.OffSetSnow`) "OffSet" (make `LinearColor` _returnvalue_x _returnvalue_y 0.0 1.0))
  ;[1 1 1] 将RT材质整个绘制上去
  (`KismetRenderingLibrary.DrawMaterialToRenderTarget` "/Game/Material/RenderTarget/InteractSnow/RT_Snow.RT_Snow" (`self.OffSetSnow`))
  (bind (_canvas _size _context) (`KismetRenderingLibrary.BeginDrawCanvasToRenderTarget` "/Game/Material/RenderTarget/InteractSnow/RT_Snow.RT_Snow"))
  (for _array_element (`self.Brush Info`)
    (`MaterialInstanceDynamic.SetScalarParameterValue` _drawsnowmaterial "Height" (- 1.0 (/ (- _snowheight (`.Height_9_E26D345742E8898E47C00F945602938B` (break `/Game/Material/RenderTarget/InteractSnow/S_BrushInfo` _array_element))) _snowheight)))
    (bind _returnvalue (* (`.Size_5_89885DC14F85462CF6FAD19413FA3D5C` (break `/Game/Material/RenderTarget/InteractSnow/S_BrushInfo` _array_element)) (0.5 0.5)))
    (`Canvas.K2_DrawMaterial` _canvas _drawsnowmaterial (- (* _size (`self.WorldLocationToRT_UV` (break `/Game/Material/RenderTarget/InteractSnow/S_BrushInfo` _array_element))) (/ _returnvalue (2.0 2.0))) _returnvalue (0.0 0.0) (1.0 1.0) 0.0 (0.5 0.5)))
  (`KismetRenderingLibrary.EndDrawCanvasToRenderTarget` _context)
  (`KismetArrayLibrary.Array_Clear` (`self.Brush Info`))
  (`KismetRenderingLibrary.DrawMaterialToRenderTarget` "/Game/Material/RenderTarget/InteractSnow/RT_SnowSave.RT_SnowSave" "/Game/Material/RenderTarget/InteractSnow/M_Accumulation.M_Accumulation"))

(event `AddBrush`
  (params (BrushInfo :type "/Game/Material/RenderTarget/InteractSnow/S_BrushInfo Structure"))
  (`KismetArrayLibrary.Array_Add` (`self.Brush Info`) BrushInfo))

(fn `CopySnowRT`
  (bind (_canvas _size _context) (`KismetRenderingLibrary.BeginDrawCanvasToRenderTarget` "/Game/Material/RenderTarget/InteractSnow/RT_SnowSave.RT_SnowSave"))
  (`Canvas.K2_DrawTexture` _canvas "/Game/Material/RenderTarget/InteractSnow/RT_Snow.RT_Snow" (0.0 0.0) _size (0.0 0.0) (1.0 1.0) (struct :`R` 1.0 :`G` 1.0 :`B` 1.0 :`A` 1.0) "BLEND_Opaque" 0.0 (0.5 0.5))
  (`KismetRenderingLibrary.EndDrawCanvasToRenderTarget` _context))

(fn `UpdatePosition`
  (params (Pos :type "Vector2D Structure"))
  (bind (_position_x _position_y) (`KismetMathLibrary.BreakVector2D` (`self.Position`)))
  (bind (_canvassize_x _canvassize_y) (`KismetMathLibrary.BreakVector2D` (`self.CanvasSize`)))
  (set `self.LastPosition` (`self.Position`))
  (set `self.Position` Pos)
  (`KismetMaterialLibrary.SetVectorParameterValue` "/Game/Material/RenderTarget/InteractSnow/MPC_Snow.MPC_Snow" "PositionAndSize" (make `LinearColor` _position_x _position_y _canvassize_x _canvassize_y)))

(fn `UserConstructionScript`)

(fn `WorldLocationToRT_UV`
  (params (Location :type "Vector Structure"))
  (returns (NewParam :type "Vector2D Structure"))
  (return (+ (/ (- (`KismetMathLibrary.MakeVector2D` (.x Location) (.y Location)) (`self.Position`)) (`self.CanvasSize`)) (0.5 0.5))))
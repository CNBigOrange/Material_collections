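; Fluid canvas actor that maintains a render target centered on the player pawn, stamped with brushes at world locations.
; Each tick it publishes position and canvas size to a material parameter collection, then clears BufferB and redraws M_FluidBufferB with the normalized movement offset.
; Brushes queued through AddBrush are converted to canvas UVs, drawn, then emptied.
; The copy from BufferB to BufferB_Save is disconnected.
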(event `self.ReceiveBeginPlay`
  (`KismetRenderingLibrary.ClearRenderTarget2D` "/Game/Material/Fluid/BufferB_Save.BufferB_Save")
  (`KismetRenderingLibrary.ClearRenderTarget2D` "/Game/Material/Fluid/BufferB.BufferB")
  (bind _returnvalue (`KismetMaterialLibrary.CreateDynamicMaterialInstance` "/Game/Material/Fluid/M_FluidBufferB.M_FluidBufferB"))
  (set `self.OffsetBuffer` _returnvalue))

(event `self.ReceiveTick`
  (params (DeltaSeconds :type "Float (single-precision)"))
  (bind (_position_x _position_y) (`KismetMathLibrary.BreakVector2D` (`self.Position`)))
  (bind (_canvassize_x _canvassize_y) (`KismetMathLibrary.BreakVector2D` (`self.CanvasSize`)))
  (bind (_returnvalue_x _returnvalue_y) (`KismetMathLibrary.BreakVector2D` (/ (- (`self.Position`) (`self.LastPosition`)) (`self.CanvasSize`))))
  ;[1 1 1] Comment
  (set `self.LastPosition` (`self.Position`))
  (set `self.Position` (`KismetMathLibrary.Conv_VectorToVector2D` (`self.K2_GetActorLocation` (`GameplayStatics.GetPlayerPawn` 0))))
  (`KismetMaterialLibrary.SetVectorParameterValue` "/Game/Material/Fluid/MPC_Paramters.MPC_Paramters" "PositionAndSize" (make `LinearColor` _position_x _position_y _canvassize_x _canvassize_y))
  (`KismetRenderingLibrary.ClearRenderTarget2D` "/Game/Material/Fluid/BufferB.BufferB")
  (`MaterialInstanceDynamic.SetVectorParameterValue` (`self.OffsetBuffer`) "OffSet" (make `LinearColor` _returnvalue_x _returnvalue_y 0.0 1.0))
  (`KismetRenderingLibrary.DrawMaterialToRenderTarget` "/Game/Material/Fluid/BufferB.BufferB" (`self.OffsetBuffer`))
  (bind (_canvas _size _context) (`KismetRenderingLibrary.BeginDrawCanvasToRenderTarget` "/Game/Material/Fluid/BufferB.BufferB"))
  (for _array_element (`self.BrushInfo`)
    (`Canvas.K2_DrawTexture` _canvas null (- (* _size (`self.WorldLocationToRT_UV` (break `/Game/Material/RenderTarget/InteractSnow/S_BrushInfo` _array_element))) (/ (* (`.Size_5_89885DC14F85462CF6FAD19413FA3D5C` (break `/Game/Material/RenderTarget/InteractSnow/S_BrushInfo` _array_element)) (0.5 0.5)) (2.0 2.0))) (`.Size_5_89885DC14F85462CF6FAD19413FA3D5C` (break `/Game/Material/RenderTarget/InteractSnow/S_BrushInfo` _array_element)) (0.0 0.0) (1.0 1.0) (struct :`R` 1.0 :`G` 1.0 :`B` 1.0 :`A` 1.0) "BLEND_Translucent" 0.0 (0.5 0.5)))
  (`KismetRenderingLibrary.EndDrawCanvasToRenderTarget` _context)
  (`KismetArrayLibrary.Array_Clear` (`self.BrushInfo`)))

(event `AddBrush`
  (params (NewParam :type "/Game/Material/RenderTarget/InteractSnow/S_BrushInfo Structure"))
  (`KismetArrayLibrary.Array_Add` (`self.BrushInfo`) NewParam))

(fn `UserConstructionScript`)

(fn `WorldLocationToRT_UV`
  (params (NewParam :type "Vector Structure"))
  (returns (NewParam1 :type "Vector2D Structure"))
  (return (+ (/ (- (`KismetMathLibrary.MakeVector2D` (.x NewParam) (.y NewParam)) (`self.Position`)) (`self.CanvasSize`)) (0.5 0.5))))